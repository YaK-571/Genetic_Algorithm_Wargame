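; Squad actor for a wargame that spawns a team's units in a 5x5 battle formation and relocates to an assigned point.
; After a spawn delay, BeginPlay reads each cell's unit type from the game instance by team (Comanda) and squad (Otdelenie).
; FSpawn places a tank, BTR, car or soldier at the cell's slot and passes it team, squad and position.
; The squad then teleports to BpPoint; Event_AI_MoveTo later lerps it there by Timeline.
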(event Custom|Event_test)

(event Custom|Event_AI_MoveTo
  (bind _bp_point (Variables|Default|Getbp_point))
  ;[1 1 1] Перемещение отделения
  (Variables|Default|Setstart_location (Transformation|GetActorLocation))
  (Utilities|IsValid _bp_point
    (:Is%20Valid
      (Variables|Default|Setfinal_location (Transformation|GetActorLocation _bp_point))
      (bind _newtrack_0 (Timeline|Timeline Play)
        (:Update
          (Transformation|SetActorLocation (Math|Vector|Lerp(Vector) (Variables|Default|Getstart_location) (Variables|Default|Getfinal_location) _newtrack_0) false true))))))

(event EventBeginPlay
  (bind _otdelenie (Variables|Default|Getotdelenie))
  (bind _bp_point (Variables|Default|Getbp_point))
  (bind _returnvalue (- _otdelenie 1))
  (bind _asbp_game_instance_wargame (Utilities|Casting|CastToBP_Game_Instance_Wargame (Game|GetGameInstance)))
  (Variables|Default|SetAs%20BP%20Game%20Instance%20Wargame _asbp_game_instance_wargame)
  (Utilities|FlowControl|Delay (Variables|Default|Getvremja_spawna))
  (for _index (range 0 4)
    (for _index_2 (range 0 4)
      (if (== (Variables|Default|Getcomanda) 1)
        (bind _returnvalue_2 (Class|GameInstanceWargame|FGetSquad (Variables|Default|GetAs%20BP%20Game%20Instance%20Wargame) _returnvalue _index _index_2))
        (Variables|Default|Settip_int _returnvalue_2)
        (else
          (bind _returnvalue_3 (Class|GameInstanceWargame|FGetSquad2 (Variables|Default|GetAs%20BP%20Game%20Instance%20Wargame) _returnvalue _index _index_2))
          (Variables|Default|Settip_int _returnvalue_3)))
      (switch int _index
        (:0
          (switch int _index_2
            (:0
              (Variables|Default|Setmesto (Variables|Default|Get1_0)))
            (:1
              (Variables|Default|Setmesto (Variables|Default|Get1_1)))
            (:2
              (Variables|Default|Setmesto (Variables|Default|Get1_2)))
            (:3
              (Variables|Default|Setmesto (Variables|Default|Get1_3)))
            (:4
              (Variables|Default|Setmesto (Variables|Default|Get1_4)))))
        (:1
          (switch int _index_2
            (:0
              (Variables|Default|Setmesto (Variables|Default|Get2_0)))
            (:1
              (Variables|Default|Setmesto (Variables|Default|Get2_1)))
            (:2
              (Variables|Default|Setmesto (Variables|Default|Get2_2)))
            (:3
              (Variables|Default|Setmesto (Variables|Default|Get2_3)))
            (:4
              (Variables|Default|Setmesto (Variables|Default|Get2_4)))))
        (:2
          (switch int _index_2
            (:0
              (Variables|Default|Setmesto (Variables|Default|Get3_0)))
            (:1
              (Variables|Default|Setmesto (Variables|Default|Get3_1)))
            (:2
              (Variables|Default|Setmesto (Variables|Default|Get3_2)))
            (:3
              (Variables|Default|Setmesto (Variables|Default|Get3_3)))
            (:4
              (Variables|Default|Setmesto (Variables|Default|Get3_4)))))
        (:3
          (switch int _index_2
            (:0
              (Variables|Default|Setmesto (Variables|Default|Get4_0)))
            (:1
              (Variables|Default|Setmesto (Variables|Default|Get4_1)))
            (:2
              (Variables|Default|Setmesto (Variables|Default|Get4_2)))
            (:3
              (Variables|Default|Setmesto (Variables|Default|Get4_3)))
            (:4
              (Variables|Default|Setmesto (Variables|Default|Get4_4)))))
        (:4
          (switch int _index_2
            (:0
              (Variables|Default|Setmesto (Variables|Default|Get5_0)))
            (:1
              (Variables|Default|Setmesto (Variables|Default|Get5_1)))
            (:2
              (Variables|Default|Setmesto (Variables|Default|Get5_2)))
            (:3
              (Variables|Default|Setmesto (Variables|Default|Get5_3)))
            (:4
              (Variables|Default|Setmesto (Variables|Default|Get5_4))))))
      (CallFunction|FSpawn (Variables|Default|Getmesto) (Variables|Default|Gettip_int))))
  (Utilities|IsValid _bp_point
    (:Is%20Valid
      (Transformation|SetActorLocation (Transformation|GetActorLocation _bp_point) false true))))

(event Collision|EventActorBeginOverlap
  (params (OtherActor :type Actor%20Object%20Reference)))

(event EventTick
  (params (DeltaSeconds :type Float%20%28single-precision%29)))

(fn ConstructionScript)

(fn FSpawn
  (params (component :type Scene%20Component%20Object%20Reference) (tip :type Integer))
  (bind _returnvalue (Transformation|GetWorldRotation component))
  (switch int tip
    (:1
      (Variables|Default|Settip "/Game/Blueprint/BP_Armor_Tank.BP_Armor_Tank_C"))
    (:2
      (Variables|Default|Settip "/Game/Blueprint/BP_BTR.BP_BTR_C"))
    (:3
      (Variables|Default|Settip "/Game/Blueprint/BP_car.BP_car_C"))
    (:4
      (Variables|Default|Settip "/Game/Blueprint/BP_soldier.BP_soldier_C")))
  (bind _returnvalue_2 (Game|SpawnActorfromClass (Variables|Default|Gettip) (Math|Transform|MakeTransform (Transformation|GetWorldLocation component) (Math|Rotator|MakeRotator (.roll _returnvalue) (.pitch _returnvalue) (+ (.yaw _returnvalue) 9e+01)) "1.000000,1.000000,1.000000") "AlwaysSpawn" "MultiplyWithRoot" 0 0))
  (Variables|/Game/Blueprint/BP_NPC_abstract.BP_NPC_abstract_C|Setcomanda _returnvalue_2 (Variables|Default|Getcomanda))
  (Variables|/Game/Blueprint/BP_NPC_abstract.BP_NPC_abstract_C|Setotdelenie _returnvalue_2 (Variables|Default|Getotdelenie))
  (Variables|/Game/Blueprint/BP_NPC_abstract.BP_NPC_abstract_C|Setposizija _returnvalue_2 (Variables|Default|Getmesto))
  (Default|EventSpawnController _returnvalue_2))

(fn FGetSquad
  (params (otdelenie :type Integer))
  (for _index (range 0 4)
    (for _index_2 (range 0 4)
      (bind _returnvalue (Class|Squad|FGetBattleFormation otdelenie _index _index_2))
      (return _returnvalue _index _index_2))))