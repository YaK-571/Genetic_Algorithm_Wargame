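; Soldier NPC Blueprint that extends a parent unit, adding target-based weapon choice and the ability to occupy buildings.
; On a target change, it picks burst-fire soldier projectiles if the enemy's class matches ClassActor, otherwise slower single RPG shots.
; On the enter event, it moves to the target house's entrance; if unclaimed, the house takes its team and scaled HP, and the soldier is destroyed.
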(event Custom|Event_vhod
  (bind _target_house (Variables|Default|Gettarget_house))
  ;[1 1 1] Вход в здание
  (AI|AIMoveTo self (Transformation|GetWorldLocation (Variables|/Game/Blueprint/BP_bunker.BP_bunker_C|GetScene_vhod (Variables|Default|Gettarget_house))) 0 15.0 false
    (:OnSuccess
      (if (== (Variables|/Game/Blueprint/BP_bunker.BP_bunker_C|Getcomanda _target_house) 0)
        (Variables|/Game/Blueprint/BP_bunker.BP_bunker_C|Setcomanda _target_house (Variables|Default|Getcomanda))
        (Variables|/Game/Blueprint/BP_bunker.BP_bunker_C|Sethp _target_house (* (Variables|Default|GetHP) 20))
        (Default|EventVhod _target_house)
        (Actor|DestroyActor)))))

(event EventBeginPlay
  (|CallParentFunction) ; This node is disabled and will not be called.\nDrag off pins to build functionality.
)

(event Collision|EventActorBeginOverlap
  (params (OtherActor :type Actor%20Object%20Reference))
  (|CallParentFunction OtherActor) ; This node is disabled and will not be called.\nDrag off pins to build functionality.
)

(event EventTick
  (params (DeltaSeconds :type Float%20%28single-precision%29))
  (|CallParentFunction DeltaSeconds) ; This node is disabled and will not be called.\nDrag off pins to build functionality.
)

(event EventEventSmenaZeli
  ;[1 1 1] Разное оружие в зависимости от вида противника
  (|CallParentFunction)
  (if (== (Utilities|GetClass (Variables|Default|GetNPC_vrag)) (Variables|Default|GetClass_actor))
    (Variables|Default|SetBP_ball "/Game/Blueprint/ball/BP_ball_coldier.BP_ball_coldier_C")
    (Variables|Default|Setskorostrelnost 3.0)
    (Variables|Default|Setotschered_max 3)
    (Variables|Default|Setskorostrelnost_otschered 0.2)
    (else
      (Variables|Default|SetBP_ball "/Game/Blueprint/ball/BP_ball_coldier_rpg.BP_ball_coldier_rpg_C")
      (Variables|Default|Setskorostrelnost 5.0)
      (Variables|Default|Setotschered_max 1)
      (Variables|Default|Setskorostrelnost_otschered 1.0))))

(fn ConstructionScript
  (|CallParentFunction))