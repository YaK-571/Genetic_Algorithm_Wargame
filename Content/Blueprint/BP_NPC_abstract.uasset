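; Base team-based NPC combat unit that moves to an assigned position, spots enemies and picks targets, with empty attack and detected events.
; On start it links its AI controller, BP_camera and same-team units.
; Each tick it rebuilds detected enemies using sight radii per camouflage level, shares sightings with allies and, lacking a target, selects one within firing range.
; It also toggles selection highlighting, and reports points to BP_camera before destruction at zero HP.
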(event Custom|Event_spawn_controller
  (bind _posizija (Variables|Default|Getposizija))
  (Pawn|SpawnDefaultController)
  ;[1 1 1] Получение ссылки на собственный контроллер
  (bind _asai_controller_my (Utilities|Casting|CastToAI_Controller_my (AI|GetAIController self)))
  (bind _output_get (Variables|Default|SetAs%20AI%20Controller%20My _asai_controller_my))
  (Variables|/Game/AI/AI_Controller_my.AI_Controller_my_C|SetNPC_self _output_get self)
  (Variables|Default|Setmaskirovka (Variables|Default|Getmaskirovka_max))
  (bind _outactors (Actor|GetAllActorsOfClass "/Game/Blueprint/BP_camera.BP_camera_C"))
  (Variables|Default|SetBP_camera (Utilities|Array|Get(acopy) _outactors))
  (CallFunction|EventSvoi)
  ;[1 1 1] Движение до точки
  (Utilities|IsValid _posizija
    (:Is%20Valid
      (Utilities|FlowControl|Delay 0.5)
      (Variables|Default|Setzel (Transformation|GetWorldLocation _posizija))
      (CallFunction|EventAIMoveto))))

(event Custom|Event_AI_MoveTo
  ;[1 1 1] Движение
  (AI|AIMoveTo self (Variables|Default|Getzel) 0 1e+01 false
    (:OnSuccess
      (Utilities|IsValid (Variables|Default|Getposizija)
        (:Is%20Valid
          _)))
    (:OnFail
      (Utilities|FlowControl|Delay 5.0)))
  (CallFunction|EventAIMoveto))

(event Custom|Event_sbros_vudelenija
  ;[1 1 1] Подсветка юнита, если он выделен
  (Rendering|Material|SetMaterial (Variables|Default|GetCube) 0 "/Game/Material/M_zvet7_beszvettuj.M_zvet7_beszvettuj"))

(event Custom|Event_vudelenie
  ;[1 1 1] Подсветка юнита, если он выделен
  (Rendering|Material|SetMaterial (Variables|Default|GetCube) 0 "/Game/Material/M_zvet6.M_zvet6"))

(event Custom|Event_Damage
  (bind _bp_camera (Variables|Default|GetBP_camera))
  (bind _ballu (Variables|Default|Getballu))
  (bind _comanda (Variables|Default|Getcomanda))
  ;[1 1 1] Получение урона
  (if (<= (Variables|Default|GetHP) 0)
    (Default|FBallu _bp_camera _comanda (Variables|Default|Getotdelenie_vraga) _ballu)
    (Default|FBallu2 _bp_camera _comanda (Variables|Default|Getotdelenie) _ballu)
    (Actor|DestroyActor)))

(event Custom|Event_skorost
  ;[1 1 1] Изменение скорости
  (Variables|/Script/Engine.CharacterMovementComponent|SetMaxWalkSpeed (Variables|Character|GetCharacterMovement) (Variables|Default|Getskorost)))

(event Custom|Event_Ataka)

(event Custom|Event_NPC_obnaruschen)

(event Custom|Event_vrag_minus
  ;[1 1 1] Удаление из массива уничтоженной техники
  (Utilities|Array|RemoveItem (Variables|Default|Getvse_vragi_obnaruschennue_mnoj) (Variables|Default|GetNPC_vrag))
  (Variables|Default|SetNPC_vrag 0)
  (CallFunction|EventSmenaZeli))

(event Custom|Event_smena_zeli
  (bind _vse_vragi_obnaruschennue_mnoj (Variables|Default|Getvse_vragi_obnaruschennue_mnoj))
  ;[1 1 1] Сделать целью последний валидный обьект в массиве
  (Utilities|IsValid (Variables|Default|GetNPC_vrag)
    (:Is%20Not%20Valid
      (for _array_element _vse_vragi_obnaruschennue_mnoj
        (Utilities|IsValid _array_element
          (:Is%20Valid
            (if (< (Math|Vector|VectorLength (- (Transformation|GetActorLocation _array_element) (Transformation|GetActorLocation))) (Variables|Default|Getdalnost_strelbu))
              (Variables|Default|SetNPC_vrag _array_element)))
          (:Is%20Not%20Valid
            ;;[1 1 1] Удали из массива уничтоженного противника
            (Utilities|Array|RemoveItem _vse_vragi_obnaruschennue_mnoj _array_element))))
      ;[1 1 1] Если список целей не пуст - продолжать атаку
      (if (> (Utilities|Array|Length (Variables|Default|Getvse_vragi_obnaruschennue_mnoj)) 0)
        (Utilities|IsValid (Variables|Default|GetNPC_vrag)
          (:Is%20Valid
            (Variables|Default|SetAtaka false)
            (CallFunction|EventAtaka))
          (:Is%20Not%20Valid
            (Variables|Default|SetAtaka false :!label _label)
            (CallFunction|EventSkorost)))
        (else
          (goto _label))))))

(event Custom|Event_test
  (bind _test2 (Variables|Default|Gettest2))
  (Utilities|IsValid _test2
    (:Is%20Valid
      (Development|PrintString (Utilities|String|ToString(Float) (Math|Vector|VectorLength (- (Transformation|GetActorLocation _test2) (Transformation|GetActorLocation))))))))

(event Custom|Event_svoi
  ;[1 1 1] Получение ссылок на тиммейтов
  (bind _outactors (Actor|GetAllActorsOfClass "BP_NPC_abstract_C"))
  (for _array_element _outactors
    (if (== (Variables|BP_NPC_abstract_C|Getcomanda _array_element) (Variables|Default|Getcomanda))
      (Utilities|Array|Add (Variables|Default|Getvse_svoi) _array_element))))

(event EventBeginPlay
  (bind _posizija (Variables|Default|Getposizija))
  ;[1 0 0] BEGIN PLAY
  ;[1 1 1] Получение ссылки на собственный контроллер
  (bind _asai_controller_my (Utilities|Casting|CastToAI_Controller_my (AI|GetAIController self)))
  (bind _output_get (Variables|Default|SetAs%20AI%20Controller%20My _asai_controller_my))
  (Variables|/Game/AI/AI_Controller_my.AI_Controller_my_C|SetNPC_self _output_get self)
  (Variables|Default|Setmaskirovka (Variables|Default|Getmaskirovka_max))
  (bind _outactors (Actor|GetAllActorsOfClass "/Game/Blueprint/BP_camera.BP_camera_C"))
  (Variables|Default|SetBP_camera (Utilities|Array|Get(acopy) _outactors))
  (CallFunction|EventSvoi)
  ;[1 1 1] Движение до точки
  (Utilities|IsValid _posizija
    (:Is%20Valid
      (Utilities|FlowControl|Delay 0.5)
      (Variables|Default|Setzel (Transformation|GetWorldLocation _posizija))
      (CallFunction|EventAIMoveto))))

(event Collision|EventActorBeginOverlap
  (params (OtherActor :type Actor%20Object%20Reference)))

(event EventTick
  (params (DeltaSeconds :type Float%20%28single-precision%29))
  (Utilities|Array|Clear (Variables|Default|Getvse_vragi_obnaruschennue_mnoj))
  (CallFunction|EventTest)
  ;[1 1 1] Измерение дальности до врагов для их засвета
  (for _array_element (Variables|Default|Getvse_vragi)
    (Utilities|IsValid _array_element
      (:Is%20Valid
        (if (Math|Boolean|ORBoolean (and (== (Variables|BP_NPC_abstract_C|Getmaskirovka _array_element) 1) (< (Math|Vector|VectorLength (- (Transformation|GetActorLocation _array_element) (Transformation|GetActorLocation))) (Variables|Default|Getobzor_1))) (and (== (Variables|BP_NPC_abstract_C|Getmaskirovka _array_element) 2) (< (Math|Vector|VectorLength (- (Transformation|GetActorLocation _array_element) (Transformation|GetActorLocation))) (Variables|Default|Getobzor_2))) (and (== (Variables|BP_NPC_abstract_C|Getmaskirovka _array_element) 3) (< (Math|Vector|VectorLength (- (Transformation|GetActorLocation _array_element) (Transformation|GetActorLocation))) (Variables|Default|Getobzor_3))))
          (CallFunction|FObnafuschenie _array_element)
          (CallFunction|EventNPCObnaruschen _array_element)
          ;[1 1 1] Передача информации об обнаруженом враге всем союзникам
          (for _array_element_2 (Variables|Default|Getvse_svoi)
            (Utilities|IsValid _array_element_2
              (:Is%20Valid
                (CallFunction|FSvjas _array_element_2 _array_element))))))))
  (CallFunction|EventSmenaZeli))

(fn ConstructionScript)

(fn FObnafuschenie
  (params (NewParam :type BP%20NPC%20Abstract%20Object%20Reference))
  (if (not (Utilities|Array|ContainsItem (Variables|Default|Getvse_vragi_obnaruschennue_mnoj) NewParam))
    (Utilities|Array|Add (Variables|Default|Getvse_vragi_obnaruschennue_mnoj) NewParam)
    ;[1 1 1] Если это первая обнаруженная цель - начни атаку
    (if (not (Variables|Default|GetAtaka))
      (CallFunction|EventSmenaZeli))))

(fn FSvjas
  (params (NewParam :type BP%20NPC%20Abstract%20Object%20Reference))
  (if (Utilities|Array|ContainsItem (Variables|Default|Getvse_vragi) NewParam)
    (if (not (Utilities|Array|ContainsItem (Variables|Default|Getvse_vragi_obnaruschennue_mnoj) NewParam))
      (Utilities|Array|Add (Variables|Default|Getvse_vragi_obnaruschennue_mnoj) NewParam)
      ;[1 1 1] Если это первая обнаруженная цель - начни атаку
      (if (not (Variables|Default|GetAtaka))
        (CallFunction|EventSmenaZeli)))))