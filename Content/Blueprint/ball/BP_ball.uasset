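; BP_ball is a projectile that damages NPCs derived from BP_NPC_abstract and destroys itself when its sphere overlaps an actor.
; Damage reduces HP only when the target's Bronja (armor) does not exceed the ball's Bronebojnost (penetration).
; On a lethal hit it passes its Otdelenie (squad) to the victim, calls EventDamage, and notifies a valid SelfTank through EventVragMinus.
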(event OnComponentBeginOverlap(Sphere)
  (params (OverlappedComponent :type Primitive%20Component%20Object%20Reference) (OtherActor :type Actor%20Object%20Reference) (OtherComp :type Primitive%20Component%20Object%20Reference) (OtherBodyIndex :type Integer) (bFromSweep :type Boolean) (SweepResult :type Hit%20Result%20Structure%20%28by%20ref%29))
  (bind _self_tank (Variables|Default|Getself_tank))
  (bind _asbp_npc_abstract (Utilities|Casting|CastToBP_NPC_abstract OtherActor)
    (:then
      (if (<= (Variables|/Game/Blueprint/BP_NPC_abstract.BP_NPC_abstract_C|Getbronja _asbp_npc_abstract) (Variables|Default|Getbronebojnost))
        (bind _output_get (Variables|/Game/Blueprint/BP_NPC_abstract.BP_NPC_abstract_C|SetHP _asbp_npc_abstract (- (Variables|/Game/Blueprint/BP_NPC_abstract.BP_NPC_abstract_C|GetHP _asbp_npc_abstract) (Variables|Default|GetDamage))))
        (if (> _output_get 0)
          _
          (else
            (Variables|/Game/Blueprint/BP_NPC_abstract.BP_NPC_abstract_C|Setotdelenie_vraga _asbp_npc_abstract (Variables|Default|Getotdelenie))
            (Default|EventDamage _asbp_npc_abstract)
            (Utilities|IsValid _self_tank
              (:Is%20Valid
                (Default|EventVragMinus _self_tank))
              (:Is%20Not%20Valid
                _))))))
    (:CastFailed
      _))
  (Actor|DestroyActor))

(event EventBeginPlay)

(event Collision|EventActorBeginOverlap
  (params (OtherActor :type Actor%20Object%20Reference)))

(event EventTick
  (params (DeltaSeconds :type Float%20%28single-precision%29)))

(fn ConstructionScript)