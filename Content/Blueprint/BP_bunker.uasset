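; Bunker building that a soldier can occupy and leave, with a highlight material toggled for selection.
; Entering spawns an embrasure linked to the bunker and its team (Comanda), with its own controller.
; Exiting an occupied bunker spawns a team soldier with a fifth of bunker HP, then resets team and HP and destroys the embrasure.
; Damage only subtracts HP; the eviction call in that function is unconnected.
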(event OnComponentBeginOverlap(Cube)
  (params (OverlappedComponent :type Primitive%20Component%20Object%20Reference) (OtherActor :type Actor%20Object%20Reference) (OtherComp :type Primitive%20Component%20Object%20Reference) (OtherBodyIndex :type Integer) (bFromSweep :type Boolean) (SweepResult :type Hit%20Result%20Structure%20%28by%20ref%29)))

(event Custom|Event_vudelenie
  (Rendering|Material|SetMaterial (Variables|Default|Getvudelenie) 0 "/Game/Material/M_zvet6.M_zvet6"))

(event Custom|Event_otmena_vudelenija
  (Rendering|Material|SetMaterial (Variables|Default|Getvudelenie) 0 "/Game/Material/M_zvet7_beszvettuj.M_zvet7_beszvettuj"))

(event Custom|Event_vhod
  (Utilities|Array|Clear (Variables|Default|Getboinizu))
  (CallFunction|FSpawn (Transformation|GetWorldTransform (Variables|Default|Get1))))

(event Custom|Event_vuhod
  ;[1 1 1] Выход из здания
  (if (!= (Variables|Default|Getcomanda) 0)
    (bind _returnvalue (Game|SpawnActorfromClass "/Game/Blueprint/BP_soldier.BP_soldier_C" (Math|Transform|MakeTransform (Transformation|GetWorldLocation (Variables|Default|GetScene_vhod)) "0, 0, 0" "1.000000,1.000000,1.000000") "AlwaysSpawn" "MultiplyWithRoot" 0 0))
    (Utilities|IsValid _returnvalue
      (:Is%20Valid
        (Variables|/Game/Blueprint/BP_NPC_abstract.BP_NPC_abstract_C|SetHP _returnvalue (/ (Variables|Default|Gethp) 5))
        (Variables|/Game/Blueprint/BP_NPC_abstract.BP_NPC_abstract_C|Setcomanda _returnvalue (Variables|Default|Getcomanda))
        (Default|EventSpawnController _returnvalue)
        (CallFunction|FVuhod)))))

(event EventBeginPlay
  (CallFunction|EventOtmenaVudelenija))

(event Collision|EventActorBeginOverlap
  (params (OtherActor :type Actor%20Object%20Reference)))

(event EventTick
  (params (DeltaSeconds :type Float%20%28single-precision%29)))

(fn ConstructionScript)

(fn FSpawn
  (params (SpawnTransform :type Transform))
  (bind _returnvalue (Game|SpawnActorfromClass "/Game/Blueprint/BP_embrasure.BP_embrasure_C" (Math|Transform|MakeTransform (.location SpawnTransform) (.rotation SpawnTransform) "1.000000,1.000000,1.000000") "AlwaysSpawn" "MultiplyWithRoot" 0 0))
  (Utilities|IsValid _returnvalue
    (:Is%20Valid
      (Variables|/Game/Blueprint/BP_embrasure.BP_embrasure_C|Sethouse _returnvalue self)
      (Variables|/Game/Blueprint/BP_NPC_abstract.BP_NPC_abstract_C|Setcomanda _returnvalue (Variables|Default|Getcomanda))
      (Default|EventSpawnController _returnvalue)
      (Utilities|Array|Add (Variables|Default|Getboinizu) _returnvalue))))

(fn FVuhod
  (bind _boinizu (Variables|Default|Getboinizu))
  (bind _output (Utilities|Array|Get(acopy) _boinizu))
  (Variables|Default|Setcomanda 0)
  (Variables|Default|Sethp 0)
  (Utilities|IsValid _output
    (:Is%20Valid
      (Default|EventDamage _output))
    (:Is%20Not%20Valid
      _))
  (for _array_element _boinizu
    (Utilities|IsValid _array_element
      (:Is%20Valid
        (Actor|DestroyActor _array_element))))
  (Utilities|Array|Clear (Variables|Default|Getboinizu)))

(fn FDamage
  (params (NewParam :type Integer))
  (Variables|Default|Sethp (- (Variables|Default|Gethp) NewParam)))