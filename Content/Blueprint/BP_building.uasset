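; BP_building is a child building Blueprint that extends its parent's EventVhod and EventVuhod events (transliterated Russian for entrance and exit).
; On EventVhod it runs the parent logic, then calls FSpawn at the world transforms of three marker references named 2, 3 and 4.
; EventVuhod and the construction script only forward to the parent, and BeginPlay, overlap and Tick are disabled stubs.
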(event EventBeginPlay
  (|CallParentFunction) ; This node is disabled and will not be called.\nDrag off pins to build functionality.
)

(event Collision|EventActorBeginOverlap
  (params (OtherActor :type Actor%20Object%20Reference))
  (|CallParentFunction OtherActor) ; This node is disabled and will not be called.\nDrag off pins to build functionality.
)

(event EventTick
  (params (DeltaSeconds :type Float%20%28single-precision%29))
  (|CallParentFunction DeltaSeconds) ; This node is disabled and will not be called.\nDrag off pins to build functionality.
)

(event EventEventVuhod
  (|CallParentFunction))

(event EventEventVhod
  (|CallParentFunction)
  (CallFunction|FSpawn (Transformation|GetWorldTransform (Variables|Default|Get2)))
  (CallFunction|FSpawn (Transformation|GetWorldTransform (Variables|Default|Get3)))
  (CallFunction|FSpawn (Transformation|GetWorldTransform (Variables|Default|Get4))))

(fn ConstructionScript
  (|CallParentFunction))