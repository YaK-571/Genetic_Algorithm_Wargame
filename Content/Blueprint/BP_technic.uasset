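; Tank NPC child Blueprint handling team color, enemy visibility and turret combat.
; Non-team-2 units start hidden and are revealed on detection, which also signals their lamp widget.
; Attacks check target armor against penetration, halt movement, then swing the turret on a timeline rate-scaled by angle and aim speed.
; It fires BPBall bursts with random spread, reloads and re-attacks, switching targets when one is invalid or too armored.
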(event Custom|Event_zvet
  (bind _korpus (Variables|Default|Getkorpus))
  ;[1 1 1] Цвет команды
  (switch int (Variables|Default|Getcomanda)
    (:1
      (Variables|Default|SetNew_material "/Game/Material/M_zvet3_blue.M_zvet3_blue")
      (Rendering|Material|SetMaterial _korpus 0 (Variables|Default|GetNew_material)))
    (:2
      (Variables|Default|SetNew_material "/Game/Material/M_zvet1_red.M_zvet1_red")
      (Rendering|Material|SetMaterial _korpus 0 (Variables|Default|GetNew_material)))))

(event Custom|Event_vustrel
  (bind _scene (Variables|Default|GetScene))
  (bind _metkost (Variables|Default|Getmetkost))
  (bind _metkost_2 (Variables|Default|Getmetkost))
  (bind _metkost_3 (Variables|Default|Getmetkost))
  (bind _npc_vrag (Variables|Default|GetNPC_vrag))
  (bind _returnvalue (Transformation|GetActorLocation _npc_vrag))
  (bind _returnvalue_2 (Transformation|GetWorldTransform _scene))
  ;[1 1 1] Выстрел
  (Utilities|IsValid (Variables|Default|GetNPC_vrag) :!label _label
    (:Is%20Valid
      ;;[1 1 1] Рассеивание
      (Math|Integer|IncrementInt (Variables|Default|Getotschered)
        (:%20%20
          (Transformation|SetWorldRotation (Variables|Default|GetScene) (Math|Rotator|FindLookatRotation (Transformation|GetWorldLocation (Variables|Default|GetScene)) (Math|Vector|MakeVector (+ (.x _returnvalue) (Math|Random|RandomFloatinRange (* _metkost_2 -1.0) _metkost_2)) (+ (.y _returnvalue) (Math|Random|RandomFloatinRange (* _metkost_3 -1.0) _metkost_3)) (+ (.z _returnvalue) (Math|Random|RandomFloatinRange (* _metkost -1.0) _metkost)))) false false)
          (bind _returnvalue_3 (Game|SpawnActorfromClass (Variables|Default|GetBP_ball) (Math|Transform|MakeTransform (.location _returnvalue_2) (.rotation _returnvalue_2) "1.000000,1.000000,1.000000") "AlwaysSpawn" "MultiplyWithRoot" 0 0))
          (Utilities|IsValid _returnvalue_3
            (:Is%20Valid
              (Variables|/Game/Blueprint/ball/BP_ball.BP_ball_C|Setself_NPC _returnvalue_3 self)
              (Variables|/Game/Blueprint/ball/BP_ball.BP_ball_C|Setotdelenie _returnvalue_3 (Variables|Default|Getotdelenie)))
            (:Is%20Not%20Valid
              _))
          (if (<= (Variables|Default|Getotschered) (Variables|Default|Getotschered_max))
            (Utilities|FlowControl|Delay (Variables|Default|Getskorostrelnost_otschered))
            (goto _label)
            (else
              (Variables|Default|Setotschered 0)
              (CallFunction|EventPerezarjadka))))))
    (:Is%20Not%20Valid
      (CallFunction|EventSmenaZeli))))

(event Custom|Event_perezarjadka
  ;[1 1 1] Перезарядка
  (Variables|Default|Setperezarjadka false)
  (Utilities|FlowControl|Delay (Variables|Default|Getskorostrelnost))
  (Variables|Default|Setperezarjadka true)
  (Utilities|IsValid (Variables|Default|GetNPC_vrag)
    (:Is%20Valid
      (CallFunction|EventAtaka))
    (:Is%20Not%20Valid
      (CallFunction|EventSmenaZeli))))

(event Custom|Event_vidimost
  ;[1 0 0] Скрой команду врага
  (if (!= (Variables|Default|Getcomanda) 2)
    (Rendering|SetActorHiddenInGame true)
    (else
      (Rendering|SetActorHiddenInGame false))))

(event EventEventNPCObnaruschen
  ;[1 1 1] Засвет
  (bind _aswbp_lampa (Utilities|Casting|CastToWBP_lampa (UserInterface|GetWidget (Variables|Default|GetWidget_0))))
  (Default|EventObnaruschen _aswbp_lampa)
  ;[1 0 0] Скрой все вражесткие танки
  (if (!= (Variables|Default|Getcomanda) 2)
    (Rendering|SetActorHiddenInGame false)))

(event Collision|EventActorBeginOverlap
  (params (OtherActor :type Actor%20Object%20Reference)))

(event EventTick
  (params (DeltaSeconds :type Float%20%28single-precision%29)))

(event EventBeginPlay
  (|CallParentFunction)
  (CallFunction|EventSkorost)
  (CallFunction|EventZvet)
  (CallFunction|EventVidimost))

(event EventEventSpawnController
  (|CallParentFunction)
  (CallFunction|EventZvet)
  (CallFunction|EventVidimost))

(event EventEventAtaka
  (bind _npc_vrag (Variables|Default|GetNPC_vrag))
  (Variables|Default|SetAtaka true)
  (Utilities|IsValid _npc_vrag
    (:Is%20Valid
      ;[1 1 1] Доворот башни
      (if (<= (Variables|/Game/Blueprint/BP_NPC_abstract.BP_NPC_abstract_C|Getbronja _npc_vrag) (Variables|Default|Getbronebojnost))
        (Variables|/Script/Engine.CharacterMovementComponent|SetMaxWalkSpeed (Variables|Character|GetCharacterMovement) 0.0)
        (Variables|Default|Setlocation_baschnja_start (Transformation|GetWorldLocation (Variables|Default|Getbaschnja)))
        (bind _output_get (Variables|Default|Setrotate_start (Transformation|GetWorldRotation (Variables|Default|Getbaschnja))))
        (bind _output_get_2 (Variables|Default|Setrotate_zel (Math|Rotator|FindLookatRotation (Variables|Default|Getlocation_baschnja_start) (Transformation|GetActorLocation (Variables|Default|GetNPC_vrag)))))
        (if (!= (Utilities|Operators|Divide 1.8e+02 (Class|KismetMathLibrary|DegAcos (Math|Vector|DotProduct (Math|Rotator|GetRotationXVector _output_get_2) (Math|Rotator|GetRotationXVector _output_get))) (Variables|Default|Getskorost_baschnja_aim)) 0.0)
          ;[1 1 1] Длительность таймлайна
          (Components|Timeline|SetPlayRate (Variables|Default|GetTimeline_test) (Utilities|Operators|Divide 1.8e+02 (Class|KismetMathLibrary|DegAcos (Math|Vector|DotProduct (Math|Rotator|GetRotationXVector _output_get_2) (Math|Rotator|GetRotationXVector _output_get))) (Variables|Default|Getskorost_baschnja_aim)))
          (bind _newtrack_0 (Timeline|Timeline_test PlayFromStart)
            (:Update
              (Transformation|SetWorldRotation (Variables|Default|Getbaschnja) (Math|Rotator|Lerp(Rotator) (Variables|Default|Getrotate_start) (Variables|Default|Getrotate_zel) _newtrack_0 true) false false))
            (:Finished
              (if (Variables|Default|Getperezarjadka)
                (CallFunction|EventVustrel))))
          (else
            (Components|Timeline|SetPlayRate (Variables|Default|GetTimeline_test) 1e+02)
            (Timeline|Timeline_test PlayFromStart)))
        (else
          (CallFunction|EventSkorost :!label _label)
          (CallFunction|EventSmenaZeli)
          (AI|Components|Blackboard|SetValueasBool (AI|GetBlackboard 0) (Utilities|String|StringToName "ataka") false))))
    (:Is%20Not%20Valid
      (goto _label))))

(fn ConstructionScript
  (|CallParentFunction))