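; RTS camera for the wargame that also runs round scoring and restarts.
; It pans by keys or screen edges, tilts and moves vertically via the wheel, and turns clicks into HUD selection, house picking and unit move, attack or enter orders.
; Squad points accumulate in the interface widget against a victory threshold.
; On threshold or timeout, FFinish exports squad efficiency through the game instance, stores the top two squads and reloads the level.
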(event Custom|Event_podstschot_ballov
  ;[1 1 1] Подсчёт баллов
  (Utilities|FlowControl|Delay 1.0)
  (bind _outactors (Actor|GetAllActorsOfClass "/Game/Blueprint/BP_NPC_abstract.BP_NPC_abstract_C"))
  (for _array_element _outactors
    (switch int (Variables|/Game/Blueprint/BP_NPC_abstract.BP_NPC_abstract_C|Getcomanda _array_element)
      (:1
        (Variables|Default|Setmax_ball1 (+ (Variables|Default|Getmax_ball1) (Variables|/Game/Blueprint/BP_NPC_abstract.BP_NPC_abstract_C|Getballu _array_element))))
      (:2
        (Variables|Default|Setmax_ball2 (+ (Variables|Default|Getmax_ball2) (Variables|/Game/Blueprint/BP_NPC_abstract.BP_NPC_abstract_C|Getballu _array_element)))))))

(event Custom|Event_defoult_cursor
  ;[1 1 1] Изменение курсора
  (Variables|Default|Setcustom_cursor false)
  (Variables|/Script/Engine.PlayerController|SetCurrentMouseCursor (Game|GetPlayerController 0) "Default"))

(event Custom|Event_custom_cursor
  ;[1 1 1] Изменение курсора
  (Variables|Default|Setcustom_cursor true)
  (Variables|/Script/Engine.PlayerController|SetCurrentMouseCursor (Game|GetPlayerController 0) "Hand"))

(event EventBeginPlay
  ;[1 0 0] Бегин плей
  (Variables|/Script/Engine.PlayerController|SetbShowMouseCursor (Game|GetPlayerController 0) true)
  (bind _returnvalue (UserInterface|CreateWidget "/Game/Widget/WBP_interfase.WBP_interfase_C"))
  (bind _output_get (Variables|Default|SetWBP_interface _returnvalue))
  (UserInterface|Viewport|AddtoViewport _output_get 0)
  (CallFunction|EventPodstschotBallov)
  (bind _asbp_game_instance_wargame (Utilities|Casting|CastToBP_Game_Instance_Wargame (Game|GetGameInstance)))
  (bind _output_get_2 (Variables|Default|SetAs%20BP%20Game%20Instance%20Wargame _asbp_game_instance_wargame))
  (Class|GameInstanceWargame|FStart _output_get_2)
  (bind _asbp_controller_camera (Utilities|Casting|CastToBP_controller_camera (Game|GetPlayerController 0)))
  (bind _output_get_3 (Variables|Default|SetAs%20BP%20Controller%20Camera _asbp_controller_camera))
  (bind _ashud_wargame (Utilities|Casting|CastToHUD_Wargame (HUD|GetHUD _output_get_3)))
  (bind _output_get_4 (Variables|Default|SetAs%20HUD%20Wargame _ashud_wargame))
  (Variables|/Game/Widget/HUD_Wargame.HUD_Wargame_C|Setself_camera _output_get_4 self)
  ;[1 1 1] Остановить раунд по истечении некоторого времени
  (Utilities|FlowControl|Delay (Variables|Default|Getdlina_raunda))
  (CallFunction|FFinish))

(event Collision|EventActorBeginOverlap
  (params (OtherActor :type Actor%20Object%20Reference)))

(event EventTick
  (params (DeltaSeconds :type Float%20%28single-precision%29))
  (bind _returnvalue (Game|GetPlayerController 0))
  (bind _hitresult (Game|Player|GetHitResultUnderCursorbyChannel _returnvalue "TraceTypeQuery1" true))
  (if (> (Utilities|Array|Length (Variables|Default|Getvudelennui_NPC_array)) 0)
    ;[1 1 1] Если курсор наведёт на дом - выдели его
    (if (.bblockinghit _hitresult)
      (if (Variables|Default|Getpehota?)
        (bind _asbp_house (Utilities|Casting|CastToBP_house (.hitactor _hitresult))
          (:then
            (Variables|Default|Sethouse_cursore _asbp_house)
            (if (not (Variables|Default|Getcustom_cursor))
              (CallFunction|EventCustomCursor)))
          (:CastFailed
            ;[1 1 1] Если курсор наведён на врага - поменяй его
            (bind _asbp_npc_abstract (Utilities|Casting|CastToBP_NPC_abstract (.hitactor _hitresult) :!label _label)
              (:then
                (if (not (!= (Variables|/Game/Blueprint/BP_NPC_abstract.BP_NPC_abstract_C|Getcomanda _asbp_npc_abstract) 1))
                  ;[1 1 1] В иных случаях верни дефолтный курсор
                  (if (Variables|Default|Getcustom_cursor) :!label _label_2
                    (CallFunction|EventDefoultCursor))))
              (:CastFailed
                (goto _label_2)))))
        (else
          (goto _label)))
      (else
        (goto _label_2)))
    (else
      (goto _label_2))))

(event Input|ActionEvents|InputActionupr_clic1
  (params (Key :type Key%20Structure :default "None"))
  (bind _returnvalue (Game|GetPlayerController 0))
  (bind _as_hud_wargame (Variables|Default|GetAs%20HUD%20Wargame))
  (bind _hitresult (Game|Player|GetHitResultUnderCursorbyChannel _returnvalue "TraceTypeQuery1" true))
  ;[1 1 1] Выделение юнитов
  (:Pressed
    (Default|EventVudelenie _as_hud_wargame)
    ;[1 1 1] Выбор здания
    (if (.bblockinghit _hitresult)
      (Utilities|IsValid (Variables|Default|GetWBP_house)
        (:Is%20Valid
          (Widget|RemovefromParent (Variables|Default|GetWBP_house)))
        (:Is%20Not%20Valid
          _))
      (bind _asbp_house (Utilities|Casting|CastToBP_house (.hitactor _hitresult))
        (:then
          (bind _output_get (Variables|Default|SetAs%20BP%20House _asbp_house))
          (Default|EventVudelenie _output_get)
          (bind _returnvalue_2 (UserInterface|CreateWidget "/Game/Widget/WBP_house.WBP_house_C"))
          (bind _output_get_2 (Variables|Default|SetWBP_house _returnvalue_2))
          (UserInterface|Viewport|AddtoViewport _output_get_2 0)
          (Variables|/Game/Widget/WBP_house.WBP_house_C|Setbp_house _returnvalue_2 _output_get))
        (:CastFailed
          (Utilities|IsValid (Variables|Default|GetAs%20BP%20House)
            (:Is%20Valid
              (Default|EventOtmenaVudelenija (Variables|Default|GetAs%20BP%20House))
              (Variables|Default|SetAs%20BP%20House 0)))))))
  (:Released
    (Default|EventOtmenaVudelenija _as_hud_wargame)))

(event Input|ActionEvents|InputActionupr_clic2
  (params (Key :type Key%20Structure :default "None"))
  (bind _returnvalue (Game|GetPlayerController 0))
  (bind _hitresult (Game|Player|GetHitResultUnderCursorbyChannel _returnvalue "TraceTypeQuery1" true))
  (:Pressed
    (if (.bblockinghit _hitresult)
      (bind _asbp_npc_abstract (Utilities|Casting|CastToBP_NPC_abstract (.hitactor _hitresult))
        (:then
          ;[1 1 1] Если кликнули по вражесткому юниту, то атакуй его
          (for _array_element (Variables|Default|Getvudelennui_NPC_array)
            (Utilities|IsValid _array_element
              (:Is%20Valid
                (if (not (== (Variables|/Game/Blueprint/BP_NPC_abstract.BP_NPC_abstract_C|Getcomanda _asbp_npc_abstract) (Variables|/Game/Blueprint/BP_NPC_abstract.BP_NPC_abstract_C|Getcomanda _array_element)))
                  (Variables|/Game/Blueprint/BP_NPC_abstract.BP_NPC_abstract_C|SetNPC_vrag _array_element _asbp_npc_abstract)
                  (Default|EventAtaka _array_element))))))
        (:CastFailed
          (bind _asbp_house (Utilities|Casting|CastToBP_house (.hitactor _hitresult))
            (:then
              ;[1 1 1] Если цель дом - то пехота входит в него
              (if (== (Variables|/Game/Blueprint/BP_house.BP_house_C|Getcomanda _asbp_house) 0)
                (for _array_element_2 (Variables|Default|Getvudelennui_NPC_array)
                  (Utilities|IsValid _array_element_2
                    (:Is%20Valid
                      (bind _asbp_soldier (Utilities|Casting|CastToBP_soldier _array_element_2))
                      (Variables|/Game/Blueprint/BP_soldier.BP_soldier_C|Settarget_house _asbp_soldier _asbp_house)
                      (Default|EventVhod _asbp_soldier))))))
            (:CastFailed
              (for _array_element_3 (Variables|Default|Getvudelennui_NPC_array)
                (Utilities|IsValid _array_element_3
                  (:Is%20Valid
                    ;[1 1 1] Едь до выбранной точки
                    (Variables|/Game/Blueprint/BP_NPC_abstract.BP_NPC_abstract_C|Setzel _array_element_3 (.location _hitresult))
                    (Default|EventAIMoveto _array_element_3)))))))))))

(event Input|ActionEvents|InputActionupr_1
  (params (Key :type Key%20Structure :default "None")))

(event Input|AxisEvents|InputAxisupr_w
  (params (AxisValue :type Float%20%28single-precision%29))
  ;[1 1 1] Передвижение камеры
  (Transformation|AddActorWorldOffset (Math|Vector|MakeVector (* AxisValue (Utilities|Time|GetWorldDeltaSeconds) (Variables|Default|Getspeed)) 0.0 0.0) false true))

(event Input|AxisEvents|InputAxisupr_s
  (params (AxisValue :type Float%20%28single-precision%29))
  ;[1 1 1] Передвижение камеры
  (Transformation|AddActorWorldOffset (Math|Vector|MakeVector (* AxisValue -1.0 (Utilities|Time|GetWorldDeltaSeconds) (Variables|Default|Getspeed)) 0.0 0.0) false true))

(event Input|AxisEvents|InputAxisupr_a
  (params (AxisValue :type Float%20%28single-precision%29))
  ;[1 1 1] Передвижение камеры
  (Transformation|AddActorWorldOffset (Math|Vector|MakeVector 0.0 (* AxisValue (Utilities|Time|GetWorldDeltaSeconds) (Variables|Default|Getspeed) -1.0) 0.0) false true))

(event Input|AxisEvents|InputAxisupr_d
  (params (AxisValue :type Float%20%28single-precision%29))
  ;[1 1 1] Передвижение камеры
  (Transformation|AddActorWorldOffset (Math|Vector|MakeVector 0.0 (* AxisValue 1.0 (Utilities|Time|GetWorldDeltaSeconds) (Variables|Default|Getspeed)) 0.0) false true))

(event Input|AxisEvents|InputAxisupr_mouse_kolosiko
  (params (AxisValue :type Float%20%28single-precision%29))
  ;[1 1 1] Приближение и отдаление при прокрутке колёсика
  (Transformation|AddActorWorldOffset (Math|Vector|MakeVector 0.0 0.0 (* AxisValue (Utilities|Time|GetWorldDeltaSeconds) -6e+03)) false true))

(event Input|AxisEvents|InputAxisupr_mouse_y
  (params (AxisValue :type Float%20%28single-precision%29))
  (bind _returnvalue (Game|GetPlayerController 0))
  (bind _returnvalue_2 (Viewport|GetViewportSize))
  (bind _returnvalue_3 (Utilities|Time|GetWorldDeltaSeconds))
  (bind _speed (Variables|Default|Getspeed))
  (bind _locationx (Game|Player|GetMousePosition _returnvalue))
  (bind _returnvalue_4 (/ _locationx (.x _returnvalue_2)))
  ;[1 1 1] Перемещение камеры вслед за мышкой
  (if (> _returnvalue_4 0.95)
    (Transformation|AddActorWorldOffset (Math|Vector|MakeVector 0.0 (* _returnvalue_3 _speed) 0.0) false true)
    (elif (< _returnvalue_4 0.05)
      (Transformation|AddActorWorldOffset (Math|Vector|MakeVector 0.0 (* -1.0 _returnvalue_3 _speed) 0.0) false true))))

(event Input|AxisEvents|InputAxisupr_mouse_x
  (params (AxisValue :type Float%20%28single-precision%29))
  (bind _returnvalue (Game|GetPlayerController 0))
  (bind _returnvalue_2 (Viewport|GetViewportSize))
  (bind _returnvalue_3 (Utilities|Time|GetWorldDeltaSeconds))
  (bind _speed (Variables|Default|Getspeed))
  (bind _locationy (Game|Player|GetMousePosition _returnvalue))
  (bind _returnvalue_4 (/ _locationy (.y _returnvalue_2)))
  ;[1 1 1] Перемещение камеры вслед за мышкой
  (if (> _returnvalue_4 0.95)
    (Transformation|AddActorWorldOffset (Math|Vector|MakeVector (* -1.0 _returnvalue_3 _speed) 0.0 0.0) false true)
    (elif (< _returnvalue_4 0.05)
      (Transformation|AddActorWorldOffset (Math|Vector|MakeVector (* _returnvalue_3 _speed) 0.0 0.0) false true))))

(event Input|AxisEvents|InputAxisupr_mouse_kolosiko_down
  (params (AxisValue :type Float%20%28single-precision%29))
  (bind _returnvalue (Game|GetPlayerController 0))
  (bind _returnvalue_2 (Viewport|GetViewportSize))
  (bind _camera (Variables|Default|GetCamera))
  (bind _camera_2 (Variables|Default|GetCamera))
  (bind _locationy (Game|Player|GetMousePosition _returnvalue))
  (bind _relativerotation (Variables|/Script/Engine.SceneComponent|GetRelativeRotation _camera))
  (bind _returnvalue_3 (/ _locationy (.y _returnvalue_2)))
  ;[1 1 1] Наклон камеры при зажатии колёсика
  (if (== AxisValue 1.0)
    (if (> _returnvalue_3 0.6)
      (if (> (.pitch _relativerotation) -8e+01)
        (Transformation|AddRelativeRotation _camera_2 (Math|Rotator|MakeRotator 0.0 (* (Utilities|Time|GetWorldDeltaSeconds) -25.0) 0.0) false false))
      (elif (< _returnvalue_3 0.4)
        (if (< (.pitch _relativerotation) -1e+01)
          (Transformation|AddRelativeRotation _camera_2 (Math|Rotator|MakeRotator 0.0 (* (Utilities|Time|GetWorldDeltaSeconds) 25.0) 0.0) false false))))))

(fn ConstructionScript)

(fn FBallu
  (params (comanda :type Integer) (otdelenie :type Integer) (ballu :type Integer))
  (bind _wbp_interface (Variables|Default|GetWBP_interface))
  (bind _wbp_interface_2 (Variables|Default|GetWBP_interface))
  (bind _wbp_interface_3 (Variables|Default|GetWBP_interface))
  (bind _wbp_interface_4 (Variables|Default|GetWBP_interface))
  ;[1 1 1] Обновление виждета
  (Variables|Default|Setballu_1 ballu)
  (switch int comanda
    (:1
      (switch int otdelenie
        (:1
          (Variables|/Game/Widget/WBP_interfase.WBP_interfase_C|Set2_1 _wbp_interface (+ (Variables|/Game/Widget/WBP_interfase.WBP_interfase_C|Get2_1 _wbp_interface) (Variables|Default|Getballu_1))))
        (:2
          (Variables|/Game/Widget/WBP_interfase.WBP_interfase_C|Set2_2 _wbp_interface (+ (Variables|/Game/Widget/WBP_interfase.WBP_interfase_C|Get2_2 _wbp_interface) (Variables|Default|Getballu_1))))
        (:3
          (Variables|/Game/Widget/WBP_interfase.WBP_interfase_C|Set2_3 _wbp_interface (+ (Variables|/Game/Widget/WBP_interfase.WBP_interfase_C|Get2_3 _wbp_interface) (Variables|Default|Getballu_1))))
        (:4
          (Variables|/Game/Widget/WBP_interfase.WBP_interfase_C|Set2_4 _wbp_interface (+ (Variables|/Game/Widget/WBP_interfase.WBP_interfase_C|Get2_4 _wbp_interface) (Variables|Default|Getballu_1))))
        (:5
          (Variables|/Game/Widget/WBP_interfase.WBP_interfase_C|Set2_5 _wbp_interface (+ (Variables|/Game/Widget/WBP_interfase.WBP_interfase_C|Get2_5 _wbp_interface) (Variables|Default|Getballu_1)))))
      (Variables|Default|Setfact_ball2 (+ (Variables|/Game/Widget/WBP_interfase.WBP_interfase_C|Get2_1 _wbp_interface_4) (Variables|/Game/Widget/WBP_interfase.WBP_interfase_C|Get2_2 _wbp_interface_4) (Variables|/Game/Widget/WBP_interfase.WBP_interfase_C|Get2_3 _wbp_interface_4) (Variables|/Game/Widget/WBP_interfase.WBP_interfase_C|Get2_4 _wbp_interface_4) (Variables|/Game/Widget/WBP_interfase.WBP_interfase_C|Get2_5 _wbp_interface_4)))
      (if (< (/ (Variables|Default|Getmax_ball1) (Variables|Default|GetBALL_pobeda)) (Variables|Default|Getfact_ball2))
        (if (not (Variables|Default|Getfinish)) :!label _label
          (Variables|Default|Setfinish true)
          ;[1 1 1] В конце боя проверка какие отделения наиболее эффективные
          (CallFunction|FFinish))))
    (:2
      (switch int otdelenie
        (:1
          (Variables|/Game/Widget/WBP_interfase.WBP_interfase_C|Set1 _wbp_interface_3 (+ (Variables|/Game/Widget/WBP_interfase.WBP_interfase_C|Get1 _wbp_interface_3) (Variables|Default|Getballu_1))))
        (:2
          (Variables|/Game/Widget/WBP_interfase.WBP_interfase_C|Set2 _wbp_interface_3 (+ (Variables|/Game/Widget/WBP_interfase.WBP_interfase_C|Get2 _wbp_interface_3) (Variables|Default|Getballu_1))))
        (:3
          (Variables|/Game/Widget/WBP_interfase.WBP_interfase_C|Set3 _wbp_interface_3 (+ (Variables|/Game/Widget/WBP_interfase.WBP_interfase_C|Get3 _wbp_interface_3) (Variables|Default|Getballu_1))))
        (:4
          (Variables|/Game/Widget/WBP_interfase.WBP_interfase_C|Set4 _wbp_interface_3 (+ (Variables|/Game/Widget/WBP_interfase.WBP_interfase_C|Get4 _wbp_interface_3) (Variables|Default|Getballu_1))))
        (:5
          (Variables|/Game/Widget/WBP_interfase.WBP_interfase_C|Set5 _wbp_interface_3 (+ (Variables|/Game/Widget/WBP_interfase.WBP_interfase_C|Get5 _wbp_interface_3) (Variables|Default|Getballu_1)))))
      (Variables|Default|Setfact_ball1 (+ (Variables|/Game/Widget/WBP_interfase.WBP_interfase_C|Get1 _wbp_interface_2) (Variables|/Game/Widget/WBP_interfase.WBP_interfase_C|Get2 _wbp_interface_2) (Variables|/Game/Widget/WBP_interfase.WBP_interfase_C|Get3 _wbp_interface_2) (Variables|/Game/Widget/WBP_interfase.WBP_interfase_C|Get4 _wbp_interface_2) (Variables|/Game/Widget/WBP_interfase.WBP_interfase_C|Get5 _wbp_interface_2)))
      (if (< (/ (Variables|Default|Getmax_ball2) (Variables|Default|GetBALL_pobeda)) (Variables|Default|Getfact_ball1))
        (goto _label)))))

(fn FBallu2
  (params (comanda :type Integer) (otdelenie :type Integer) (ballu :type Integer))
  (bind _wbp_interface (Variables|Default|GetWBP_interface))
  (bind _wbp_interface_2 (Variables|Default|GetWBP_interface))
  (Variables|Default|Setballu_1 ballu)
  (switch int comanda
    (:1
      (switch int otdelenie
        (:1
          (Variables|/Game/Widget/WBP_interfase.WBP_interfase_C|Setkill_1 _wbp_interface (+ (Variables|/Game/Widget/WBP_interfase.WBP_interfase_C|Getkill_1 _wbp_interface) (Variables|Default|Getballu_1))))
        (:2
          (Variables|/Game/Widget/WBP_interfase.WBP_interfase_C|Setkill_2 _wbp_interface (+ (Variables|/Game/Widget/WBP_interfase.WBP_interfase_C|Getkill_2 _wbp_interface) (Variables|Default|Getballu_1))))
        (:3
          (Variables|/Game/Widget/WBP_interfase.WBP_interfase_C|Setkill_3 _wbp_interface (+ (Variables|/Game/Widget/WBP_interfase.WBP_interfase_C|Getkill_3 _wbp_interface) (Variables|Default|Getballu_1))))
        (:4
          (Variables|/Game/Widget/WBP_interfase.WBP_interfase_C|Setkill_4 _wbp_interface (+ (Variables|/Game/Widget/WBP_interfase.WBP_interfase_C|Getkill_4 _wbp_interface) (Variables|Default|Getballu_1))))
        (:5
          (Variables|/Game/Widget/WBP_interfase.WBP_interfase_C|Setkill_5 _wbp_interface (+ (Variables|/Game/Widget/WBP_interfase.WBP_interfase_C|Getkill_5 _wbp_interface) (Variables|Default|Getballu_1))))))
    (:2
      (switch int otdelenie
        (:1
          (Variables|/Game/Widget/WBP_interfase.WBP_interfase_C|Setkill_2_1 _wbp_interface_2 (+ (Variables|/Game/Widget/WBP_interfase.WBP_interfase_C|Getkill_2_1 _wbp_interface_2) (Variables|Default|Getballu_1))))
        (:2
          (Variables|/Game/Widget/WBP_interfase.WBP_interfase_C|Setkill_2_2 _wbp_interface_2 (+ (Variables|/Game/Widget/WBP_interfase.WBP_interfase_C|Getkill_2_2 _wbp_interface_2) (Variables|Default|Getballu_1))))
        (:3
          (Variables|/Game/Widget/WBP_interfase.WBP_interfase_C|Setkill_2_3 _wbp_interface_2 (+ (Variables|/Game/Widget/WBP_interfase.WBP_interfase_C|Getkill_2_3 _wbp_interface_2) (Variables|Default|Getballu_1))))
        (:4
          (Variables|/Game/Widget/WBP_interfase.WBP_interfase_C|Setkill_2_4 _wbp_interface_2 (+ (Variables|/Game/Widget/WBP_interfase.WBP_interfase_C|Getkill_2_4 _wbp_interface_2) (Variables|Default|Getballu_1))))
        (:5
          (Variables|/Game/Widget/WBP_interfase.WBP_interfase_C|Setkill_2_5 _wbp_interface_2 (+ (Variables|/Game/Widget/WBP_interfase.WBP_interfase_C|Getkill_2_5 _wbp_interface_2) (Variables|Default|Getballu_1))))))))

(fn FFinish
  (bind _wbp_interface (Variables|Default|GetWBP_interface))
  (bind _wr (Variables|Default|GetWR))
  (bind _indexofmaxvalue (Math|Float|MaxOfFloatArray _wr))
  (bind _wr_1 (Variables|/Game/Widget/WBP_interfase.WBP_interfase_C|Getwr_1 _wbp_interface))
  (bind _wr_2 (Variables|/Game/Widget/WBP_interfase.WBP_interfase_C|Getwr_2 _wbp_interface))
  (bind _wr_3 (Variables|/Game/Widget/WBP_interfase.WBP_interfase_C|Getwr_3 _wbp_interface))
  (bind _wr_4 (Variables|/Game/Widget/WBP_interfase.WBP_interfase_C|Getwr_4 _wbp_interface))
  (bind _wr_5 (Variables|/Game/Widget/WBP_interfase.WBP_interfase_C|Getwr_5 _wbp_interface))
  ;[1 1 1] В конце боя проверка какие отделения наиболее эффективные
  (Utilities|Array|Add (Variables|Default|GetWR) _wr_1)
  (Utilities|Array|Add (Variables|Default|GetWR) _wr_2)
  (Utilities|Array|Add (Variables|Default|GetWR) _wr_3)
  (Utilities|Array|Add (Variables|Default|GetWR) _wr_4)
  (Utilities|Array|Add (Variables|Default|GetWR) _wr_5)
  ;[1 1 1] Записываем кпд в экселевский файл
  (Class|GameInstanceWargame|FExcel (Variables|Default|GetAs%20BP%20Game%20Instance%20Wargame) _wr_1 _wr_2 _wr_3 _wr_4 _wr_5)
  ;[1 1 1] Записываем наиболее эффективные отделения в гейм инстанс
  (for _index (range 0 1)
    (Class|GameInstanceWargame|FSetTopSquad (Variables|Default|GetAs%20BP%20Game%20Instance%20Wargame) _index _indexofmaxvalue)
    (Utilities|Array|RemoveIndex _wr _indexofmaxvalue))
  (bind _returnvalue (Game|GetCurrentLevelName true))
  (Game|OpenLevel(byName) (Utilities|String|StringToName _returnvalue)))